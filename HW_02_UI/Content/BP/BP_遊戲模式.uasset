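; Game mode Blueprint that runs a minutes-and-seconds countdown and pauses the game when time runs out.
; Tick feeds a one-second Delay, which ignores calls while pending, so the seconds variable (秒) drops about once per second.
; When seconds fall below zero they wrap to 59 and minutes (分) decrease.
; With no minutes left, seconds reset to zero and the game pauses.
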(event `self.ReceiveTick`
  (params (DeltaSeconds :type "Float (single-precision)"))
  ;[1 0.3385 0.3385] 倒數系統
  ;;[1 1 1] 每秒秒數減一
  (`KismetSystemLibrary.Delay` 1.0) ; 延遲等待所設定的時間在執行後面的節點
  (bind _output_get (set `self.秒` (- (`self.秒`) 1)))
  ;;[1 1 1] 當秒數低於 0 就把秒數設定為59
  (if (< _output_get 0)
    (set `self.秒` 59)
    ;;[1 1 1] 分大於 0 時 分減 1
    (if (> (`self.分`) 0)
      (set `self.分` (- (`self.分`) 1))
      (else
        ;;[1 1 1] 分為 0 時  秒等於 59 就代表已經沒有時間 將秒設為0 並暫停遊戲
        (if (== (`self.秒`) 59)
          (set `self.秒` 0)
          (`GameplayStatics.SetGamePaused` true))))))

(fn `UserConstructionScript`)